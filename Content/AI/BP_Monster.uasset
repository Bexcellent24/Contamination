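; BP_Monster is an AI monster that damages the player at close range and swaps its audio to match its state.
; Overlap on DamageCollider starts a looping timer that calls DealDamage on the first-person character's health component, and leaving clears it.
; The same overlaps set the PlayerInRange flag and switch the MonsterMoving sound between attack and movement clips.
; A Scream event briefly plays a scream, then restores the movement sound.
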(event `self.DamageCollider.OnComponentBeginOverlap`
  (params (OverlappedComponent :type "PrimitiveComponent Object Reference") (OtherActor :type "Actor Object Reference") (OtherComp :type "PrimitiveComponent Object Reference") (OtherBodyIndex :type Integer) (bFromSweep :type Boolean) (SweepResult :type "HitResult Structure (by ref)"))
  (if (== OtherActor (`GameplayStatics.GetPlayerCharacter` 0))
    (`KismetSystemLibrary.K2_SetTimer` null "DealDamage" 1.0 true)
    (set `self.PlayerInRange` true)
    (`AudioComponent.SetSound` (`self.Monster_moving`) "/Game/Audio/Monser/large-monster-attack-195713.large-monster-attack-195713")))

(event `self.DamageCollider.OnComponentEndOverlap`
  (params (OverlappedComponent :type "PrimitiveComponent Object Reference") (OtherActor :type "Actor Object Reference") (OtherComp :type "PrimitiveComponent Object Reference") (OtherBodyIndex :type Integer))
  (if (== OtherActor (`GameplayStatics.GetPlayerCharacter` 0))
    (`KismetSystemLibrary.K2_ClearTimer` null "DealDamage")
    (set `self.PlayerInRange` false)
    (`AudioComponent.SetSound` (`self.Monster_moving`) "/Game/Audio/Monser/Monster_moving.Monster_moving")))

(event `Scream`
  (`AudioComponent.SetSound` (`self.Monster_moving`) "/Game/Audio/Monser/Monster_screem.Monster_screem")
  (`KismetSystemLibrary.Delay` 3.0)
  (`AudioComponent.SetSound` (`self.Monster_moving`) "/Game/Audio/Monser/Monster_moving.Monster_moving"))

(event `DealDamage`
  (bind _asbp_first_person_character (cast `/Game/FirstPerson/Blueprints/BP_FirstPersonCharacter` (`GameplayStatics.GetPlayerCharacter` 0)))
  (`/Game/MyBlueprints/Components/BP_HealthComponent.TakeDamage` (`/Game/FirstPerson/Blueprints/BP_FirstPersonCharacter.BP_HealthComponent` _asbp_first_person_character) 10.0))

(fn `UserConstructionScript`)
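; BP_ValveAdjustment is a repair Blueprint for a valve that animates turning when fixed.
; Its fix animation event plays a tightening sound and runs a timeline that yaws the static mesh 180 degrees from its current rotation.
; When the timeline finishes it hides the paper sprite, while the interrupt event stops the timeline, leaving the valve partway turned.
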(event `ItemFixAnimation`
  (bind _startrotation (`self.StartRotation`))
  (bind (_relativerotation_roll _relativerotation_pitch _relativerotation_yaw) (`KismetMathLibrary.BreakRotator` (`SceneComponent.RelativeRotation` (`self.StaticMesh`))))
  (`GameplayStatics.PlaySound2D` "/Game/Audio/Tools/Valve_Tightening.Valve_Tightening" 1.0 1.0 0.0 null null)
  (set `self.StartRotation` _relativerotation_yaw)
  (bind (_direction _valvefloat) (`Timeline|AdjustValveTimeline` :!via `PlayFromStart` :!label _label)
    (:`Update`
      (`SceneComponent.K2_SetRelativeRotation` (`self.StaticMesh`) (`KismetMathLibrary.MakeRotator` 0.0 0.0 (`KismetMathLibrary.Lerp` _startrotation (+ _startrotation 180.0) _valvefloat)) false false))
    (:`Finished`
      (`SceneComponent.SetVisibility` (`self.PaperSprite`) false false))))

(event `InterruptFixAnimation`
  (goto _label :!via `Stop`))

(fn `UserConstructionScript`
  (`parent.UserConstructionScript`))
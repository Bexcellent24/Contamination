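; BP_LeakFix is a repairable leaking pipe that starts with an active water effect and running-water audio.
; TempFix reduces the leak's velocity and swaps to a leaking sound, while ProperFix reveals the new pipe, hides the broken mesh and circle, and clears leak and audio.
; Separate animation events play duct-tape or pipe-fix montages on the player with a 2D sound, using IsAnimating and fixed delays to block overlapping plays.
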(event `self.ReceiveBeginPlay`
  (`ActorComponent.SetActive` (`self.Water_Leak`) true false)
  (`SceneComponent.SetVisibility` (`self.NewPipe`) false false)
  (`NiagaraComponent.SetVariableFloat` (`self.Water_Leak`) "VelocitySpeed" 500.0)
  (`AudioComponent.SetSound` (`self.Audio`) "/Game/Audio/Enironment/Running_Water_Pipe.Running_Water_Pipe"))

(event `ProperFix`
  (`SceneComponent.SetVisibility` (`self.NewPipe`) true false)
  (`SceneComponent.SetVisibility` (`self.StaticMesh`) false false)
  (`ActorComponent.SetActive` (`self.Water_Leak`) false false)
  (`AudioComponent.SetSound` (`self.Audio`) null)
  (`SceneComponent.SetVisibility` (`self.YelloCircle`) false false))

(event `TempFix`
  (`NiagaraComponent.SetVariableFloat` (`self.Water_Leak`) "VelocitySpeed" 200.0)
  (`AudioComponent.SetSound` (`self.Audio`) "/Game/Audio/Enironment/Leaking_Pipe.Leaking_Pipe"))

(event `TempFixAnimation`
  (if (not (`self.IsAnimating`))
    (set `self.IsAnimating` true)
    (bind _asbp_first_person_character (cast `/Game/FirstPerson/Blueprints/BP_FirstPersonCharacter` (`GameplayStatics.GetPlayerCharacter` 0)))
    (`|PlayMontage` (`Character.Mesh` _asbp_first_person_character) "/Game/Animations/Player/Fixes/M_DuctTape.M_DuctTape"
      (:`then`
        (`GameplayStatics.PlaySound2D` "/Game/Audio/Tools/Duct_Tape.Duct_Tape" 1.0 1.0 0.0 null null)
        (`KismetSystemLibrary.Delay` 2.0)
        (set `self.IsAnimating` false)))))

(event `RealFixAnimation`
  (if (not (`self.IsAnimating`))
    (set `self.IsAnimating` true)
    (bind _asbp_first_person_character (cast `/Game/FirstPerson/Blueprints/BP_FirstPersonCharacter` (`GameplayStatics.GetPlayerCharacter` 0)))
    (`|PlayMontage` (`Character.Mesh` _asbp_first_person_character) "/Game/Animations/Player/Fixes/PlayerPipeFix_Montage.PlayerPipeFix_Montage"
      (:`then`
        (`GameplayStatics.PlaySound2D` "/Game/Audio/Tools/Fixing_Pipe.Fixing_Pipe" 1.0 1.0 0.0 null null)
        (`KismetSystemLibrary.Delay` 2.5)
        (set `self.IsAnimating` false)))))

(fn `UserConstructionScript`
  (`parent.UserConstructionScript`))
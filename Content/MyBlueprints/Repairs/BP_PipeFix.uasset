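; BP_PipeFix is a repairable pipe with temporary and real fix animation events for the first-person character.
; BeginPlay hides the replacement mesh and sets the repair type on BPRepairComponent.
; Both fix events, guarded by IsAnimating, play the same montage and sound, then set the player's PlayingSpecialAnim after a delay.
; RealFixPartChange reveals the replacement mesh and hides the original connector and red circle.
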(event `TempFixAnimation`
  (if (not (`self.IsAnimating`))
    (set `self.IsAnimating` true)
    (bind _asbp_first_person_character (cast `/Game/FirstPerson/Blueprints/BP_FirstPersonCharacter` (`GameplayStatics.GetPlayerCharacter` 0)))
    (`|PlayMontage` (`Character.Mesh` _asbp_first_person_character) "/Game/Animations/Player/Fixes/PlayerPipeFix_Montage.PlayerPipeFix_Montage"
      (:`then`
        (`GameplayStatics.PlaySound2D` "/Game/Audio/Tools/Fixing_Pipe.Fixing_Pipe" 1.0 1.0 0.0 null null)
        (`KismetSystemLibrary.Delay` 3.0)
        (set `/Game/FirstPerson/Blueprints/BP_FirstPersonCharacter.PlayingSpecialAnim` true _asbp_first_person_character)
        (set `self.IsAnimating` false)))))

(event `RealFixAnimation`
  (if (not (`self.IsAnimating`))
    (set `self.IsAnimating` true)
    (bind _asbp_first_person_character (cast `/Game/FirstPerson/Blueprints/BP_FirstPersonCharacter` (`GameplayStatics.GetPlayerCharacter` 0)))
    (`|PlayMontage` (`Character.Mesh` _asbp_first_person_character) "/Game/Animations/Player/Fixes/PlayerPipeFix_Montage.PlayerPipeFix_Montage"
      (:`then`
        (`GameplayStatics.PlaySound2D` "/Game/Audio/Tools/Fixing_Pipe.Fixing_Pipe" 1.0 1.0 0.0 null null)
        (`KismetSystemLibrary.Delay` 3.0)
        (set `/Game/FirstPerson/Blueprints/BP_FirstPersonCharacter.PlayingSpecialAnim` true _asbp_first_person_character)
        (set `self.IsAnimating` false)))))

(event `self.ReceiveBeginPlay`
  (`SceneComponent.SetVisibility` (`self.StaticMesh`) false false)
  (set `/Game/MyBlueprints/Components/BP_RepairComponent.RepairType` "NewEnumerator0" (`self.BP_RepairComponent`)))

(event `RealFixPartChange`
  (`SceneComponent.SetVisibility` (`self.untitled_Pipe_straight_connector_005`) false false)
  (`SceneComponent.SetVisibility` (`self.StaticMesh`) true false)
  (`SceneComponent.SetVisibility` (`self.RedCircle`) false false))

(fn `UserConstructionScript`
  (`parent.UserConstructionScript`))
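; Hold-to-interact repair component for repair actors, covering pipe repairs, leak fixes, valve adjustments and filter replacements.
; While interact is held, Tick checks repair type, fix state and equipped item, shows status messages and accumulates hold time toward temporary or proper fixes.
; CompleteRepair updates the game mode, consumes any required item and triggers owner visual changes.
; Owner casts drive type-specific animations, and leak fixes also notify the flood controller.
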(event `self.ReceiveBeginPlay`
  (bind _asbp_first_person_character (cast `/Game/FirstPerson/Blueprints/BP_FirstPersonCharacter` (`GameplayStatics.GetPlayerCharacter` 0)))
  (set `self.PlayerRef` _asbp_first_person_character)
  (bind _outactors (`GameplayStatics.GetAllActorsOfClass` "/Game/MyBlueprints/FloodingSystem/BP_FloodController.BP_FloodController_C"))
  (bind _output (`|GetArrayItem` _outactors))
  (`/Engine/EditorBlueprintResources/StandardMacros.IsValid` _output
    (:`Is Valid`
      (set `self.FloodControllerRef` _output))))

(event `BeginInteract`
  (set `self.IsHoldingInteract` true)
  (if (not (`self.IsProperFixed`))
    (`self.BeginRepairEffects`)))

(event `EndInteract`
  (set `self.IsHoldingInteract` false)
  (set `self.CurrentHoldTime` 0.0)
  (`self.StopRepairEffects`))

(event `DisplayRepaireInformation`
  (if (not (`self.IsDisplayingInformation`))
    (set `self.IsDisplayingInformation` true)
    (bind _returnvalue (`|CreateWidget` "/Game/UI/InventorySystemUI/W_InformationMessage.W_InformationMessage_C"))
    (`UserWidget.AddToViewport` _returnvalue 0)
    (`/Game/UI/InventorySystemUI/W_InformationMessage.ShowMessage` _returnvalue (`self.InformationMessage`))
    (`KismetSystemLibrary.Delay` 2.0)
    (set `self.IsDisplayingInformation` false)
    (`Widget.RemoveFromParent` _returnvalue)))

(event `self.ReceiveTick`
  (params (DeltaSeconds :type "Float (single-precision)"))
  (bind _isholdinginteract (`self.IsHoldingInteract`))
  (if _isholdinginteract
    (if (and _isholdinginteract (`self.IsProperFixed`))
      (set `self.InformationMessage` "Fixed")
      (`self.DisplayRepaireInformation`)
      (else
        (if (`self.IsTempFixed`)
          _
          (else
            _))
        (set `self.HoldingItem` (`.ItemClass_10_8E87971B4CA8FCDA8D0B57AAA43BE532` (break `/Game/Inventory/F_ItemStruct` (`/Game/Inventory/InventorySystem.GetEquippedItem ` (`/Game/FirstPerson/Blueprints/BP_FirstPersonCharacter.InventorySystem` (`self.PlayerRef`))))))
        (switch `/Game/MyBlueprints/Enumerators/ERepairType` (`self.RepairType`)
          (:`NewEnumerator0`
            (if (`self.IsTempFixed`)
              (if (== (`self.HoldingItem`) (`self.ProperFixItem`))
                (`self.BeginRealRepairEffect` :!label _label)
                (set `self.InformationMessage` "Doing Proper Fix")
                (`self.DisplayRepaireInformation`)
                (bind _completed (`self.RepaireHold` DeltaSeconds))
                (if _completed
                  (`self.CompleteRepair` true false true (`self.RepairType`) "NewEnumerator2"))
                (else
                  (`self.BeginTempRepaireEffect`)
                  (set `self.InformationMessage` "Not Holding Pipe Part")
                  (`self.DisplayRepaireInformation`)))
              (elif (== (`self.HoldingItem`) (`self.ProperFixItem`))
                (goto _label)
                (else
                  (`self.BeginTempRepaireEffect`)
                  (set `self.InformationMessage` "Doing Temp Fix")
                  (`self.DisplayRepaireInformation`)
                  (bind _completed_2 (`self.RepaireHold` DeltaSeconds))
                  (if _completed_2
                    (`self.CompleteRepair` false true false (`self.RepairType`) "NewEnumerator1"))))))
          (:`NewEnumerator1`
            (if (`self.IsTempFixed`)
              (if (== (`self.HoldingItem`) (`self.ProperFixItem`))
                (`self.BeginRealRepairEffect`)
                (set `self.InformationMessage` "Doing Proper Fix")
                (`self.DisplayRepaireInformation`)
                (bind _completed_3 (`self.RepaireHold` DeltaSeconds))
                (if _completed_3
                  (`self.CompleteRepair` true false true (`self.RepairType`) "NewEnumerator2")
                  (`/Game/MyBlueprints/FloodingSystem/BP_FloodController.ApplyFix` (`self.FloodControllerRef`) true true))
                (else
                  (set `self.InformationMessage` "Not Holding A Pipe Part")
                  (`self.DisplayRepaireInformation`)))
              (elif (== (`self.HoldingItem`) (`self.ProperFixItem`))
                (set `self.InformationMessage` "Doing Proper Fix")
                (`self.BeginRealRepairEffect`)
                (`self.DisplayRepaireInformation`)
                (bind _completed_4 (`self.RepaireHold` DeltaSeconds))
                (if _completed_4
                  (`self.CompleteRepair` true false true (`self.RepairType`) "NewEnumerator2")
                  (`/Game/MyBlueprints/FloodingSystem/BP_FloodController.ApplyFix` (`self.FloodControllerRef`) false true))
                (elif (== (`self.HoldingItem`) (`self.TempFixItem`))
                  (`self.BeginTempRepaireEffect`)
                  (set `self.InformationMessage` "Doing Temp Fix")
                  (`self.DisplayRepaireInformation`)
                  (bind _completed_5 (`self.RepaireHold` DeltaSeconds))
                  (if _completed_5
                    (`self.CompleteRepair` false true true (`self.RepairType`) "NewEnumerator1")
                    (`/Game/MyBlueprints/FloodingSystem/BP_FloodController.ApplyFix` (`self.FloodControllerRef`) false false))
                  (else
                    (set `self.InformationMessage` "Not Holding Pipe Part or Tape")
                    (`self.DisplayRepaireInformation`))))))
          (:`NewEnumerator2`
            (bind _completed_6 (`self.RepaireHold` DeltaSeconds))
            (if _completed_6
              (`self.CompleteRepair` true false false (`self.RepairType`) "NewEnumerator2")))
          (:`NewEnumerator3`
            (if (== (`self.HoldingItem`) (`self.ProperFixItem`))
              (bind _completed_7 (`self.RepaireHold` DeltaSeconds))
              (if _completed_7
                (`self.CompleteRepair` true false true (`self.RepairType`) "NewEnumerator2"))
              (else
                (set `self.InformationMessage` "Not Holding Filter")
                (`self.DisplayRepaireInformation`)))))))
    (else
      (switch `/Game/MyBlueprints/Enumerators/ERepairType` (`self.RepairType`)
        (:`NewEnumerator0`
          (set `self.Message` "Pipe Repair"))
        (:`NewEnumerator1`
          (set `self.Message` "Leak Fix"))
        (:`NewEnumerator2`
          (set `self.Message` "Valve Adjustment"))
        (:`NewEnumerator3`
          (set `self.Message` "Filter Replacement"))))))

(fn `BeginRealRepairEffect`
  (bind _returnvalue (`self.GetOwner`))
  (switch `/Game/MyBlueprints/Enumerators/ERepairType` (`self.RepairType`)
    (:`NewEnumerator0`
      (bind _asbp_pipe_fix (cast `/Game/MyBlueprints/Repairs/BP_PipeFix` _returnvalue))
      (`/Game/MyBlueprints/Repairs/BP_PipeFix.RealFixAnimation` _asbp_pipe_fix))
    (:`NewEnumerator1`
      (bind _asbp_leak_fix (cast `/Game/MyBlueprints/Repairs/BP_LeakFix` _returnvalue))
      (`/Game/MyBlueprints/Repairs/BP_LeakFix.RealFixAnimation` _asbp_leak_fix))))

(fn `BeginRepairEffects`
  (bind _returnvalue (`self.GetOwner`))
  (bind _returnvalue_2 (`|CreateWidget` "/Game/UI/RepairUI/W_RepairBar.W_RepairBar_C" null self))
  (bind _output_get (set `self.RepairBar` _returnvalue_2))
  (`UserWidget.AddToViewport` _output_get 0)
  (switch `/Game/MyBlueprints/Enumerators/ERepairType` (`self.RepairType`)
    (:`NewEnumerator1`
      (cast `/Game/MyBlueprints/Repairs/BP_LeakFix` _returnvalue))
    (:`NewEnumerator2`
      (bind _asbp_valve_adjustment (cast `/Game/MyBlueprints/Repairs/BP_ValveAdjustment` _returnvalue))
      (`/Game/MyBlueprints/Repairs/BP_ValveAdjustment.ItemFixAnimation` _asbp_valve_adjustment))
    (:`NewEnumerator3`
      (bind _asbp_filter_replacment (cast `/Game/MyBlueprints/Repairs/BP_FilterReplacment` _returnvalue))
      (`/Game/MyBlueprints/Repairs/BP_FilterReplacment.ItemFixAnimation` _asbp_filter_replacment))))

(fn `BeginTempRepaireEffect`
  (bind _returnvalue (`self.GetOwner`))
  (switch `/Game/MyBlueprints/Enumerators/ERepairType` (`self.RepairType`)
    (:`NewEnumerator0`
      (bind _asbp_pipe_fix (cast `/Game/MyBlueprints/Repairs/BP_PipeFix` _returnvalue))
      (`/Game/MyBlueprints/Repairs/BP_PipeFix.TempFixAnimation` _asbp_pipe_fix))
    (:`NewEnumerator1`
      (bind _asbp_leak_fix (cast `/Game/MyBlueprints/Repairs/BP_LeakFix` _returnvalue))
      (`/Game/MyBlueprints/Repairs/BP_LeakFix.TempFixAnimation` _asbp_leak_fix))))

(fn `CompleteRepair`
  (params (IsProperFix :type Boolean) (IsTempFix :type Boolean) (RequiredItem :type Boolean) (RepairType :type "/Game/MyBlueprints/Enumerators/ERepairType Enum" :default "NewEnumerator0") (RepairState :type "/Game/MyBlueprints/Enumerators/ERepairState Enum" :default "NewEnumerator0"))
  (bind _returnvalue (`self.GetOwner`))
  (bind _returnvalue_2 (`self.GetOwner`))
  (bind _inventorysystem (`/Game/FirstPerson/Blueprints/BP_FirstPersonCharacter.InventorySystem` (`self.PlayerRef`)))
  (set `self.IsProperFixed` IsProperFix)
  (set `self.IsTempFixed` IsTempFix)
  (bind _output_get (set `self.ItemStruct` (make `/Game/MyBlueprints/Structs/FRepairRecord` (cast `/Game/MyBlueprints/Repairs/BP_RepairActor_Base` (`self.GetOwner`) :!pure true) RepairType RepairState)))
  (`/Game/FirstPerson/Blueprints/BP_FirstPersonGameMode.RepairTargetUpdated` (cast `/Game/FirstPerson/Blueprints/BP_FirstPersonGameMode` (`GameplayStatics.GetGameMode`) :!pure true) _output_get)
  (if (`local.RequiredItem`)
    (`/Game/Inventory/InventorySystem.SERVER_Remove` _inventorysystem (`/Game/Inventory/InventorySystem.EquippedItemIndex ` _inventorysystem) false true)
    (switch `/Game/MyBlueprints/Enumerators/ERepairType` (`self.RepairType`)
      (:`NewEnumerator0`
        (switch `/Game/MyBlueprints/Enumerators/ERepairState` (`local.RepairState`)
          (:`NewEnumerator2`
            (bind _asbp_pipe_fix (cast `/Game/MyBlueprints/Repairs/BP_PipeFix` _returnvalue))
            (`/Game/MyBlueprints/Repairs/BP_PipeFix.RealFixPartChange` _asbp_pipe_fix))))
      (:`NewEnumerator1`
        (switch `/Game/MyBlueprints/Enumerators/ERepairState` (`local.RepairState`)
          (:`NewEnumerator1`
            (bind _asbp_leak_fix (cast `/Game/MyBlueprints/Repairs/BP_LeakFix` _returnvalue_2))
            (`/Game/MyBlueprints/Repairs/BP_LeakFix.TempFix` _asbp_leak_fix))
          (:`NewEnumerator2`
            (bind _asbp_leak_fix_2 (cast `/Game/MyBlueprints/Repairs/BP_LeakFix` _returnvalue_2))
            (`/Game/MyBlueprints/Repairs/BP_LeakFix.ProperFix` _asbp_leak_fix_2))))
      (:`NewEnumerator3`
        (bind _asbp_filter_replacment (cast `/Game/MyBlueprints/Repairs/BP_FilterReplacment` _returnvalue))
        (`/Game/MyBlueprints/Repairs/BP_FilterReplacment.FixFinished` _asbp_filter_replacment)))))

(fn `LookAt`
  (returns (Message :type Text))
  (return ""))

(fn `RepaireHold`
  (params (DeltaTime :type "Float (double-precision)"))
  (returns (Completed :type Boolean))
  (bind _output_get (set `self.CurrentHoldTime` (+ DeltaTime (`self.CurrentHoldTime`))))
  (if (>= _output_get (`self.HoldTimeRequired`))
    (return true)))

(fn `StopRepairEffects`
  (bind _repairbar (`self.RepairBar`))
  (`/Engine/EditorBlueprintResources/StandardMacros.IsValid` _repairbar
    (:`Is Valid`
      (`Widget.RemoveFromParent` _repairbar)
      (switch `/Game/MyBlueprints/Enumerators/ERepairType` (`self.RepairType`)
        (:`NewEnumerator2`
          (bind _asbp_valve_adjustment (cast `/Game/MyBlueprints/Repairs/BP_ValveAdjustment` (`self.GetOwner`)))
          (`/Game/MyBlueprints/Repairs/BP_ValveAdjustment.InterruptFixAnimation` _asbp_valve_adjustment))))))
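; BP_HealthComponent tracks an actor's health, with damage, healing and a settable infection drain.
; A looping timer started at BeginPlay subtracts the infection modifier unclamped, while TakeDamage clamps and plays a hurt sound on larger hits.
; Both damage paths run CheckDead, which sets IsDead and calls SewerFlooded on BP_FirstPersonGameMode at zero health.
; IsAlive returns IsDead, and GetHealthPercentage returns the missing fraction of a fixed 100.
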(event `self.ReceiveBeginPlay`
  (set `self.CurrentHealth` (`self.MaxHealth`))
  (`KismetSystemLibrary.K2_SetTimer` null "InfectionCreep" 15.0 true))

(event `InfectionCreep`
  (set `self.CurrentHealth` (- (`self.CurrentHealth`) (`self.InfectionModifier`)))
  (`self.CheckDead`))

(event `SetInfectionModifier`
  (params (InfectionMod :type "Float (double-precision)"))
  (set `self.InfectionModifier` InfectionMod))

(fn `CheckDead`
  (if (<= (`self.CurrentHealth`) 0.0)
    (set `self.IsDead` true)
    (bind _asbp_first_person_game_mode (cast `/Game/FirstPerson/Blueprints/BP_FirstPersonGameMode` (`GameplayStatics.GetGameMode`)))
    (`/Game/FirstPerson/Blueprints/BP_FirstPersonGameMode.SewerFlooded` _asbp_first_person_game_mode)))

(fn `GetHealthPercentage`
  (returns (HealthAsPercent :type "Float (double-precision)"))
  (return (- 1.0 (/ (`self.CurrentHealth`) 100.0))))

(fn `Heal`
  (params (Amount :type "Float (double-precision)"))
  (bind _maxhealth (`self.MaxHealth`))
  (bind _returnvalue (+ (`self.CurrentHealth`) Amount))
  (set `self.CurrentHealth` _returnvalue)
  (if (> _returnvalue _maxhealth)
    (set `self.CurrentHealth` _maxhealth)))

(fn `IsAlive`
  (returns (IsDead :type Boolean))
  (return (`self.IsDead`)))

(fn `TakeDamage`
  (params (Amount :type "Float (double-precision)"))
  (set `self.CurrentHealth` (`KismetMathLibrary.FClamp` (- (`self.CurrentHealth`) Amount) 0.0 (`self.MaxHealth`)))
  (if (> Amount 6.0)
    (`GameplayStatics.PlaySound2D` "/Game/Audio/PlayerActions/Hurt.Hurt" 1.0 1.0 0.0 null null))
  (`self.CheckDead`))
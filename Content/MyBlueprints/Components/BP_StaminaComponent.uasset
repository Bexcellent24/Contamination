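; Actor component that manages player sprint stamina, with clamped drain and regen functions, exhaustion checks and a percentage getter.
; Sprint input sets the sprinting flag unless the player is crouching, and drives the character's Panting audio through a bool parameter.
; Drain clears sprinting at zero and regen runs only when not sprinting; both take delta time from an external caller.
; Input bypasses the stamina check in StartSprinting.
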(event `self.ReceiveBeginPlay`
  (bind _asbp_first_person_character (cast `/Game/FirstPerson/Blueprints/BP_FirstPersonCharacter` (`GameplayStatics.GetPlayerCharacter` 0)))
  (set `self.PlayerRef` _asbp_first_person_character))

(event `EnhancedInput|/Game/FirstPerson/Input/Actions/IA_Sprint`
  (params (ActionValue :type Boolean) (ElapsedSeconds :type "Float (double-precision)") (TriggeredSeconds :type "Float (double-precision)") (InputAction :type "InputAction Object Reference" :default "/Game/FirstPerson/Input/Actions/IA_Sprint.IA_Sprint"))
  (bind _playerref (`self.PlayerRef`))
  (bind _panting (`/Game/FirstPerson/Blueprints/BP_FirstPersonCharacter.Panting` _playerref))
  (bind _panting_2 (`/Game/FirstPerson/Blueprints/BP_FirstPersonCharacter.Panting` _playerref))
  (:`Started`
    (if (not (`/Game/FirstPerson/Blueprints/BP_FirstPersonCharacter.isCrouching` (`self.PlayerRef`)))
      (set `self.IsSprinting ` true)
      (`AudioParameterControllerInterface.SetBoolParameter` _panting_2 "IsSprinting" true)
      (`AudioComponent.Play` _panting_2 0.0)))
  (:`Completed`
    (set `self.IsSprinting ` false)
    (`AudioParameterControllerInterface.SetBoolParameter` _panting "IsSprinting" false)
    (`AudioComponent.Play` _panting 0.0)))

(fn `CanUseStamina`
  (returns (CanUseStamina :type Boolean))
  (return (> (`self.CurrentStamina `) 0.0)))

(fn `DrainStamina`
  (params (DeltaTime :type "Float (double-precision)"))
  (bind _output_get (set `self.CurrentStamina ` (`KismetMathLibrary.FClamp` (- (`self.CurrentStamina `) (* DeltaTime (`self.StaminaDrainRate `))) 0.0 (`self.MaxStamina `))))
  (if (<= _output_get 0.0)
    (set `self.IsSprinting ` false)))

(fn `GetSaminaAsPercent`
  (returns (StaminaAsPercent :type "Float (double-precision)"))
  (return (/ (`self.CurrentStamina `) (`self.MaxStamina `))))

(fn `Is Exhausted`
  (returns (`Is Exhausted` :type Boolean))
  (return (<= (`self.CurrentStamina `) 0.0)))

(fn `RegenStamina`
  (params (DeltaTime :type "Float (double-precision)"))
  (if (and (== (`self.IsSprinting `) false) (< (`self.CurrentStamina `) (`self.MaxStamina `)))
    (set `self.CurrentStamina ` (`KismetMathLibrary.FClamp` (+ (`self.CurrentStamina `) (* (`self.StaminaRegenRate `) (`local.DeltaTime`))) 0.0 (`self.MaxStamina `)))))

(fn `StartSprinting`
  (if (`self.CanUseStamina`)
    (set `self.IsSprinting ` true)))

(fn `StopSprinting`
  (set `self.IsSprinting ` false))
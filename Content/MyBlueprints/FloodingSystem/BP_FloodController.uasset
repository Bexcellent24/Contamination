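; BP_FloodController drives rising sewer flood water, escalating the player's infection risk and notifying the game mode when the flood reaches its goal height.
; Tick accumulates water height from a base rate and modifier, while a looping timer moves the water surface and checks progress.
; Progress thresholds set the health component's infection modifier.
; ApplyFix lowers the rate modifier for temporary or proper fixes, crediting earlier temporary fixes and clamping at zero.
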(event `self.ReceiveBeginPlay`
  (bind _output_get (set `self.MaxFloodRate` (/ (`self.GoalFloodHight`) (`self.BaseFloodTime`))))
  (set `self.FloodRate` _output_get)
  (bind _asbp_first_person_character (cast `/Game/FirstPerson/Blueprints/BP_FirstPersonCharacter` (`GameplayStatics.GetPlayerCharacter` 0)))
  (set `self.PlayerHealthRef` _asbp_first_person_character)
  (set `self.StartLocation` (`self.K2_GetActorLocation` (`self.WaterSurface`)))
  (`KismetSystemLibrary.K2_SetTimer` null "Raise Water" 0.4 true))

(event `self.ReceiveTick`
  (params (DeltaSeconds :type "Float (single-precision)"))
  (bind _output_get (set `self.FinalFloodRate` (* (`self.FloodRate`) (`self.FloodRateModifier`))))
  (set `self.CurrentZ` (+ (* _output_get DeltaSeconds) (`self.CurrentZ`))))

(event `Raise Water`
  (bind (_startlocation_x _startlocation_y) (`KismetMathLibrary.BreakVector` (`self.StartLocation`)))
  (bind _bp_healthcomponent (`/Game/FirstPerson/Blueprints/BP_FirstPersonCharacter.BP_HealthComponent` (`self.PlayerHealthRef`)))
  (`self.K2_SetActorLocation` (`self.WaterSurface`) (`KismetMathLibrary.MakeVector` _startlocation_x _startlocation_y (`self.CurrentZ`)) false false)
  (bind _output_get (set `self.FloodProgress` (/ (`self.CurrentZ`) (`self.GoalFloodHight`))))
  (if (>= _output_get 1.0)
    (bind _asbp_first_person_game_mode (cast `/Game/FirstPerson/Blueprints/BP_FirstPersonGameMode` (`GameplayStatics.GetGameMode`)))
    (`/Game/FirstPerson/Blueprints/BP_FirstPersonGameMode.SewerFlooded` _asbp_first_person_game_mode)
    (elif (< (`self.FloodProgress`) 0.5)
      (`/Game/MyBlueprints/Components/BP_HealthComponent.SetInfectionModifier` _bp_healthcomponent 3.0)
      (elif (< (`self.FloodProgress`) 0.75)
        (`/Game/MyBlueprints/Components/BP_HealthComponent.SetInfectionModifier` _bp_healthcomponent 5.0)
        (elif (> (`self.FloodProgress`) 0.9)
          (`/Game/MyBlueprints/Components/BP_HealthComponent.SetInfectionModifier` _bp_healthcomponent 10.0))))))

(event `ApplyFix`
  (params (WasTempFixed :type Boolean) (ProperFix :type Boolean))
  (if ProperFix
    (if WasTempFixed
      (set `self.FloodRateModifier` (- (`self.FloodRateModifier`) (- (`self.ProperFixPenalty`) (`self.TempFixPenalty`))))
      (else
        (set `self.FloodRateModifier` (- (`self.FloodRateModifier`) (`self.ProperFixPenalty`)))))
    (else
      (set `self.FloodRateModifier` (- (`self.FloodRateModifier`) (`self.TempFixPenalty`)))))
  (if (< (`self.FloodRateModifier`) 0.0)
    (set `self.FloodRateModifier` 0.0)))

(fn `UserConstructionScript`)
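; BP_Antibiotics is a usable inventory item that heals the first-person player character.
; Use plays a shake sound and the meds montage on player 0, then after timed delays consumes one equipped item through the InventorySystem server call and heals via the health component.
; LookAt builds a pickup prompt from the item's data table name, while Interactwith is empty here.
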(event `/Game/Inventory/I_InteractInterface.InteractWith`
  (params (PlayerCharacter :type "/Game/FirstPerson/Blueprints/BP_FirstPersonCharacter Object Reference")))

(event `/Game/MyBlueprints/Interfaces/I_UseableItem.Use`
  (bind _asbp_first_person_character (cast `/Game/FirstPerson/Blueprints/BP_FirstPersonCharacter` (`GameplayStatics.GetPlayerCharacter` 0)))
  (`GameplayStatics.PlaySound2D` "/Game/Audio/Tools/shaking-vitamin-bottle-102774.shaking-vitamin-bottle-102774" 1.0 1.0 0.0 null null)
  (`|PlayMontage` (`Character.Mesh` _asbp_first_person_character) "/Game/Animations/Player/Items/M_PlayerMeds.M_PlayerMeds"
    (:`then`
      (`KismetSystemLibrary.Delay` 2.0)
      (`GameplayStatics.PlaySound2D` "/Game/Audio/Tools/shaking-vitamin-bottle-102774.shaking-vitamin-bottle-102774" 1.0 1.0 0.0 null null)
      (`KismetSystemLibrary.Delay` 2.0)
      (bind _inventorysystem (`/Game/FirstPerson/Blueprints/BP_FirstPersonCharacter.InventorySystem` _asbp_first_person_character))
      (`/Game/Inventory/InventorySystem.SERVER_Remove` _inventorysystem (`/Game/Inventory/InventorySystem.EquippedItemIndex ` _inventorysystem) false true)
      (`/Game/MyBlueprints/Components/BP_HealthComponent.Heal` (`/Game/FirstPerson/Blueprints/BP_FirstPersonCharacter.BP_HealthComponent` _asbp_first_person_character) 30.0))))

(fn `LookAt`
  (returns (Message :type Text))
  (bind (_itemid_datatable _itemid_rowname) (break `DataTableRowHandle` (`/Game/Inventory/ItemDataComponent.ItemID` (`self.ItemDataComponent`))))
  (bind _returnvalue (`|GetDataTableRow` _itemid_datatable _itemid_rowname)
    (:`then`
      (return (`|FormatText` "Pick up {item} 'E' " (`.Name_2_54CA21144CCB11F988170A9183163E2E` (break `/Game/Inventory/F_ItemStruct` _returnvalue)))))))

(fn `UserConstructionScript`
  (`parent.UserConstructionScript`))
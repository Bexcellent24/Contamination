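; Flashlight actor that can be switched on and off and offers a pickup prompt when looked at.
; Use plays a switch sound and flip-flops the SpotLight intensity between lit and dark, with the light set dark at BeginPlay.
; LookAt finds the item's data table row through the ItemDataComponent's ID and returns a formatted pickup prompt with the item name.
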(event `self.ReceiveBeginPlay`
  (`LightComponent.SetIntensity` (`self.SpotLight`) 0.0))

(event `/Game/MyBlueprints/Interfaces/I_UseableItem.Use`
  (bind _spotlight (`self.SpotLight`))
  (`GameplayStatics.PlaySound2D` "/Engine/VREditor/Sounds/UI/Flashlight_Switch.Flashlight_Switch" 1.0 1.0 0.0 null null)
  (`/Engine/EditorBlueprintResources/StandardMacros.FlipFlop`
    (:`A`
      (`LightComponent.SetIntensity` _spotlight 350.0))
    (:`B`
      (`LightComponent.SetIntensity` _spotlight 0.0))))

(fn `LookAt`
  (returns (Message :type Text))
  (bind (_itemid_datatable _itemid_rowname) (break `DataTableRowHandle` (`/Game/Inventory/ItemDataComponent.ItemID` (`self.ItemDataComponent`))))
  (bind _returnvalue (`|GetDataTableRow` _itemid_datatable _itemid_rowname)
    (:`then`
      (return (`|FormatText` "Pick up {item} 'E' " (`.Name_2_54CA21144CCB11F988170A9183163E2E` (break `/Game/Inventory/F_ItemStruct` _returnvalue)))))))

(fn `UserConstructionScript`
  (`parent.UserConstructionScript`))
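; BP_Ducttape is a duct tape item actor that supplies a pick-up prompt when looked at.
; LookAt uses the data table and row name from its ItemDataComponent's ItemID to fetch the item's name and format it into the "E" key prompt.
; The event graph and construction script add no logic, and the file contains no pickup handling itself.
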(fn `LookAt`
  (returns (Message :type Text))
  (bind (_itemid_datatable _itemid_rowname) (break `DataTableRowHandle` (`/Game/Inventory/ItemDataComponent.ItemID` (`self.ItemDataComponent`))))
  (bind _returnvalue (`|GetDataTableRow` _itemid_datatable _itemid_rowname)
    (:`then`
      (return (`|FormatText` "Pick up {item} 'E' " (`.Name_2_54CA21144CCB11F988170A9183163E2E` (break `/Game/Inventory/F_ItemStruct` _returnvalue)))))))

(fn `UserConstructionScript`
  (`parent.UserConstructionScript`))